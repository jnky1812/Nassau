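; Inventory component for the first-person character that stores item structs and toggles the inventory screen.
; AddItem stacks by name and posts a HUD notification, appending new items only when that HUD widget is valid.
; RemoveItem decrements a stack by one or by the given amount, deleting depleted entries.
; The input action creates or removes WB_Inventory, switching cursor, input mode and sound, and BeginPlay grants starter Wood after a delay.
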(event Custom|Close%20Inventory
  (bind _returnvalue (Game|GetPlayerController 0))
  ;[0.196 0.7188 0.1909] Open and close inventory
  ;;[0.196 0.7188 0.1909] Close
  (Widget|RemovefromParent (Variables|Default|GetInventory%20Widget))
  (Variables|Default|SetInventory%20Widget 0)
  (Variables|/Script/Engine.PlayerController|SetbShowMouseCursor _returnvalue false)
  (Input|SetInputModeGameOnly _returnvalue false)
  (Audio|PlaySound2D "/Engine/VREditor/Sounds/UI/Dockable_Window_Close.Dockable_Window_Close" 1.0 1.0 0.0 0 0))

(event Input|EnhancedActionEvents|EnhancedInputActionIA_Inventory
  (params (ActionValue :type Boolean) (ElapsedSeconds :type Float%20%28double-precision%29) (TriggeredSeconds :type Float%20%28double-precision%29) (InputAction :type Input%20Action%20Object%20Reference :default "/Game/FirstPerson/Input/Actions/IA_Inventory.IA_Inventory"))
  (bind _returnvalue (Game|GetPlayerController 0))
  (bind _returnvalue_2 (Game|GetPlayerController 0))
  ;[0.196 0.7188 0.1909] Open and close inventory
  (:Started
    (Variables|Default|GetInventory%20Widget
      (:then
        ;;[0.196 0.7188 0.1909] Close
        (Widget|RemovefromParent (Variables|Default|GetInventory%20Widget))
        (Variables|Default|SetInventory%20Widget 0)
        (Variables|/Script/Engine.PlayerController|SetbShowMouseCursor _returnvalue_2 false)
        (Input|SetInputModeGameOnly _returnvalue_2 false)
        (Audio|PlaySound2D "/Engine/VREditor/Sounds/UI/Dockable_Window_Close.Dockable_Window_Close" 1.0 1.0 0.0 0 0))
      (:else
        (bind _returnvalue_3 (UserInterface|CreateWidget "/Game/UI/Inventory/WB_Inventory.WB_Inventory_C"))
        (bind _output_get (Variables|Default|SetInventory%20Widget _returnvalue_3))
        (UserInterface|Viewport|AddtoViewport _output_get 0)
        (Variables|/Script/Engine.PlayerController|SetbShowMouseCursor _returnvalue true)
        (Input|SetInputModeGameandUI _returnvalue 0 "DoNotLock" true false)
        (Audio|PlaySound2D "/Engine/VREditor/Sounds/UI/Dockable_Window_Open.Dockable_Window_Open" 1.0 1.0 0.0 0 0)))))

(event EventBeginPlay
  (bind _asbp_first_person_character (Utilities|Casting|CastToBP_FirstPersonCharacter (Components|GetOwner)))
  (Variables|Default|SetFirst%20Person%20Character%20BP _asbp_first_person_character)
  (Utilities|FlowControl|Delay 2.0)
  (CallFunction|AddItem (Utilities|Struct|MakeS_Item "Wood" 2 "/Engine/EditorMeshes/Cascade/BackgroundCube.BackgroundCube" "/Game/StarterContent/Textures/T_Wood_Floor_Walnut_D.T_Wood_Floor_Walnut_D")))

(fn AddItem
  (params (New%20Item :type S%20Item%20Structure))
  (bind (_name _amount _staticmesh _icon) (Utilities|Struct|BreakS_Item New%20Item))
  (bind (_name_2 _amount_2 _staticmesh_2 _icon_2 _cancraft_ _weight) (Utilities|Struct|BreakS_Item New%20Item))
  (bind (_array_element _array_index) (Utilities|Array|ForEachLoopwithBreak (Variables|Default|GetItems) :!label _label)
    (:LoopBody
      ;[0.196 0.7188 0.1909] Stack Item
      (if (Utilities|Enum|Equal(Enum) (.Name (Utilities|Struct|BreakS_Item _array_element)) _name_2)
        (Utilities|Array|SetArrayElem (Variables|Default|GetItems) _array_index (Utilities|Struct|MakeS_Item _name_2 (+ (.Amount (Utilities|Struct|BreakS_Item _array_element)) _amount_2) _staticmesh_2 _icon_2 _cancraft_ _weight))
        (LocalVariables|SetExisting%20Item? true)
        (goto _label Break)))
    (:Completed
      ;[0.196 0.7188 0.1909] Item Notification
      (bind _hud_widget (Variables|/Game/Blueprints/BPC_Stats.BPC_Stats_C|GetHUD%20Widget (Variables|/Game/FirstPerson/Blueprints/BP_FirstPersonCharacter.BP_FirstPersonCharacter_C|GetBPC_Stats (Variables|Default|GetFirst%20Person%20Character%20BP)))
        (:then
          (Default|AddItemNotification _hud_widget _name _icon _amount)
          ;[0.196 0.7188 0.1909] New Item
          (if (not (LocalVariables|GetExisting%20Item?))
            (Utilities|Array|Add (Variables|Default|GetItems) New%20Item)))
        (:else)))))

(fn RemoveItem
  (params (Item :type S%20Item%20Structure) (Decrease%20One%20Only? :type Boolean))
  (bind (_name _amount) (Utilities|Struct|BreakS_Item Item))
  (bind (_name_2 _amount_2 _staticmesh _icon _cancraft_ _weight) (Utilities|Struct|BreakS_Item Item))
  (bind (_array_element _array_index) (Utilities|Array|ForEachLoopwithBreak (Variables|Default|GetItems) :!label _label)
    (:LoopBody
      (LocalVariables|SetCurrentItemIndex _array_index)
      (if (Utilities|Enum|Equal(Enum) (.Name (Utilities|Struct|BreakS_Item _array_element)) _name)
        (if (< (.Amount (Utilities|Struct|BreakS_Item _array_element)) 2)
          _
          (elif (> (- (.Amount (Utilities|Struct|BreakS_Item _array_element)) (Math|Integer|SelectInt 1 _amount Decrease%20One%20Only?)) 0)
            (Utilities|Array|SetArrayElem (Variables|Default|GetItems) (LocalVariables|GetCurrentItemIndex) (Utilities|Struct|MakeS_Item _name_2 (- (.Amount (Utilities|Struct|BreakS_Item _array_element)) (Math|Integer|SelectInt 1 _amount Decrease%20One%20Only?)) _staticmesh _icon _cancraft_ _weight))
            (Development|PrintString (Utilities|String|ToString(Integer) (- (.Amount (Utilities|Struct|BreakS_Item _array_element)) (Math|Integer|SelectInt 1 _amount Decrease%20One%20Only?))))
            (goto _label Break)
            (else
              _)))
        (Utilities|Array|RemoveIndex (Variables|Default|GetItems) (LocalVariables|GetCurrentItemIndex))
        (Utilities|FlowControl|Sequence
          (:then_0
            (goto _label Break))
          (:then_1
            (return true)))))))