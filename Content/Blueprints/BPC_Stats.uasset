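; Player stats component that manages health, hunger, thirst and stamina and creates the HUD.
; Looping timers feed AdjustStat, which clamps each by-ref stat, updates its bar, and triggers DamagePlayer when hunger or thirst empties.
; DamagePlayer disables healing and plays throttled hit animation and sound, or ragdolls the character and opens the Island level at zero health.
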(event Custom|Damage%20Player
  (params (Amount :type Float%20%28double-precision%29))
  (bind _hud_widget (Variables|Default|GetHUD%20Widget))
  ;[0.196 0.7188 0.1909] Damage Player
  (Variables|Default|Setheal? false)
  (CallFunction|AdjustStat (Variables|Default|Gethealth) (* Amount -1.0) 1e+02 false 0.05 (Variables|/Game/UI/WB_Stats.WB_Stats_C|GetHealthBar (Variables|/Game/UI/WB_Hud.WB_Hud_C|GetWB_Stats (Variables|Default|GetHUD%20Widget))))
  (if (<= (Variables|Default|Gethealth) 0.0)
    (Default|Ragdoll (Variables|Default|GetFirst%20Person%20Character))
    (Utilities|FlowControl|Delay 3.0)
    (Game|OpenLevel(byName) "Island")
    (else
      (Utilities|FlowControl|DoOnce false :!label _label
        (:Completed
          (UserInterface|Animation|PlayAnimation _hud_widget (Variables|/Game/UI/WB_Hud.WB_Hud_C|GetDamage _hud_widget) 0.0 1 "Forward" 1.0 false)
          (Audio|PlaySoundatLocation "/Game/Audio/Charector/MS_Damage.MS_Damage" (Transformation|GetActorLocation (Components|GetOwner)) "0, 0, 0" 1.0 1.0 0.0 0 0 0 0)
          (Utilities|FlowControl|Delay 0.5)
          (goto _label Reset))))))

(event Custom|Regain%20Stamina
  ;[0.196 0.7188 0.1909] Set Stat Timers
  (if (Variables|Default|GetregainStamina?)
    (CallFunction|AdjustStat (Variables|Default|Getstamina) 0.2 1e+02 false 0.05 (Variables|/Game/UI/WB_Stats.WB_Stats_C|GetStaminaBar (Variables|/Game/UI/WB_Hud.WB_Hud_C|GetWB_Stats (Variables|Default|GetHUD%20Widget))))))

(event Custom|Heal
  ;[0.196 0.7188 0.1909] Set Stat Timers
  (if (Variables|Default|Getheal?)
    (CallFunction|AdjustStat (Variables|Default|Gethealth) 0.02 1e+02 false 0.05 (Variables|/Game/UI/WB_Stats.WB_Stats_C|GetHealthBar (Variables|/Game/UI/WB_Hud.WB_Hud_C|GetWB_Stats (Variables|Default|GetHUD%20Widget))))))

(event Custom|Drain%20Hunger
  ;[0.196 0.7188 0.1909] Set Stat Timers
  (CallFunction|AdjustStat (Variables|Default|Gethunger) -0.0005 1e+02 true 0.05 (Variables|/Game/UI/WB_Stats.WB_Stats_C|GetHungerBar (Variables|/Game/UI/WB_Hud.WB_Hud_C|GetWB_Stats (Variables|Default|GetHUD%20Widget)))))

(event Custom|Drain%20Thirst
  ;[0.196 0.7188 0.1909] Set Stat Timers
  (CallFunction|AdjustStat (Variables|Default|Getthirst) -0.005 1e+02 true 0.05 (Variables|/Game/UI/WB_Stats.WB_Stats_C|GetThirstBar (Variables|/Game/UI/WB_Hud.WB_Hud_C|GetWB_Stats (Variables|Default|GetHUD%20Widget)))))

(event EventBeginPlay
  ;[0.196 0.7188 0.1909] Set Stat Timers
  (Utilities|Time|SetTimerbyEvent (delegate Custom|Heal) 0.01 true)
  (Utilities|Time|SetTimerbyEvent (delegate Custom|Drain%20Hunger) 0.01 true)
  (Utilities|Time|SetTimerbyEvent (delegate Custom|Drain%20Thirst) 0.01 true)
  (Utilities|Time|SetTimerbyEvent (delegate Custom|Regain%20Stamina) 0.01 true)
  (bind _asbp_first_person_character (Utilities|Casting|CastToBP_FirstPersonCharacter (Components|GetOwner)))
  (Variables|Default|SetFirst%20Person%20Character _asbp_first_person_character)
  (bind _returnvalue (UserInterface|CreateWidget "/Game/UI/WB_Hud.WB_Hud_C"))
  (bind _output_get (Variables|Default|SetHUD%20Widget _returnvalue))
  (UserInterface|Viewport|AddtoViewport _output_get 0))

(fn AdjustStat
  (params (Stat :type Float%20%28double-precision%29%20%28by%20ref%29) (Amount :type Float%20%28double-precision%29) (Max%20Value :type Float%20%28double-precision%29) (Damage%20Player? :type Boolean) (Damage%20Amount :type Float%20%28double-precision%29) (Bar%20Widget :type Progress%20Bar%20Object%20Reference))
  (bind _returnvalue (+ Stat Amount))
  (bind _returnvalue_2 (Math|Float|Clamp(Float) _returnvalue 0.0 Max%20Value))
  (|SetBy-RefVar Stat _returnvalue_2)
  (CallFunction|UpdateStatBar _returnvalue_2 Max%20Value Bar%20Widget)
  (if (not (> _returnvalue_2 0.0))
    (if Damage%20Player?
      (CallFunction|DamagePlayer Damage%20Amount))))

(fn UpdateStatBar
  (params (Stat :type Float%20%28double-precision%29) (Max%20Value :type Float%20%28double-precision%29) (Bar%20Widget :type Progress%20Bar%20Object%20Reference))
  (Progress|SetPercent Bar%20Widget (/ Stat Max%20Value)))